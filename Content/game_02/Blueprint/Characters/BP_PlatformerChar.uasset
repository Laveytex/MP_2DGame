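; 2D platformer character Blueprint that handles the character's defeat.
; CallDefeated runs once, disabling capsule collision and the movement plane constraint, then calling LaunchOnDefeat to throw the character upward and along world +Y, out of the plane.
; It also jumps the sprite animation state machine to the defeated node and resets the sprite's translucent sort priority.
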(event `CallDefeated`
  (if (not (`self.IsDefeated`))
    (set `self.IsDefeated` true)
    (`PrimitiveComponent.SetCollisionEnabled` (`self.CapsuleComponent`) "NoCollision")
    (`MovementComponent.SetPlaneConstraintEnabled` (`self.CharacterMovement`) false)
    (`self.LaunchOnDefeat`)
    (`PaperZDAnimInstance.JumpToNode` (`self.GetAnimInstance`) "JumpDefeated" "None")
    (`PrimitiveComponent.SetTranslucentSortPriority` (`self.Sprite`) 0)))

(fn `LaunchOnDefeat`
  (`self.LaunchCharacter` (+ (* (`KismetMathLibrary.Vector_Up`) (`self.DefeatUpLaunch`)) (* (0.0 1.0 0.0) (`self.Defeat Forward Launch`))) true true))

(fn `UserConstructionScript`)