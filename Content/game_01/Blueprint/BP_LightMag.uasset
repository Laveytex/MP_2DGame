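; BP_LightMag is a player-controlled Paper2D side-scroller character, a light mage that runs, jumps, attacks and casts light balls.
; Enhanced Input drives jumping and X-axis movement, turning the controller and storing facing in Dir.
; Tick picks idle, run, rise or fall flipbooks from movement unless IsAttack is set.
; Hard-bound F plays the attack flipbook; R spawns BP_Charge halfway through the cast flipbook, passes it the facing, then releases IsAttack.
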(event `self.ReceiveBeginPlay`
  (bind _asplayer_controller (cast `PlayerController` (`self.GetController`)))
  (`EnhancedInputSubsystemInterface.AddMappingContext` (pcsubsystem `EnhancedInputLocalPlayerSubsystem` _asplayer_controller) "/Game/game_01/Input/IMC_Platforming.IMC_Platforming" 0 (struct)))

(event `self.ReceiveTick`
  (params (DeltaSeconds :type "Float (single-precision)"))
  (if (not (`self.IsAttack`))
    (`self.AnimationUpdate`)))

(event `EnhancedInput|/Game/game_01/Input/Actions/IA_Jump`
  (params (ActionValue :type Boolean) (ElapsedSeconds :type "Float (double-precision)") (TriggeredSeconds :type "Float (double-precision)") (InputAction :type "InputAction Object Reference" :default "/Game/game_01/Input/Actions/IA_Jump.IA_Jump"))
  (:`Started`
    (`self.Jump`))
  (:`Completed`
    (`self.StopJumping`)))

(event `EnhancedInput|/Game/game_01/Input/Actions/IA_Move`
  (params (ActionValue :type "Float (double-precision)") (ElapsedSeconds :type "Float (double-precision)") (TriggeredSeconds :type "Float (double-precision)") (InputAction :type "InputAction Object Reference" :default "/Game/game_01/Input/Actions/IA_Move.IA_Move"))
  (bind _returnvalue (< ActionValue 0.0))
  (:`Triggered`
    (`self.AddMovementInput` (1.0 0.0 0.0) ActionValue)
    (set `self.Dir` _returnvalue)
    (`Controller.SetControlRotation` (`self.GetController`) (`KismetMathLibrary.SelectRotator` (`KismetMathLibrary.MakeRotator` 0.0 0.0 180.0) (`KismetMathLibrary.MakeRotator` 0.0) _returnvalue))))

(event `Key|F`
  (params (Key :type "Key Structure"))
  (bind _sprite (`self.Sprite`))
  (:`Pressed`
    (set `self.IsAttack` true)
    (`PaperFlipbookComponent.SetFlipbook` _sprite "/Game/game_01/PaperaAssets/Character/LightMag/Flipbook/PF_Attack_1.PF_Attack_1")
    (`KismetSystemLibrary.Delay` (`PaperFlipbookComponent.GetFlipbookLength` _sprite))
    (set `self.IsAttack` false)))

(event `Key|R`
  (params (Key :type "Key Structure"))
  (bind _sprite (`self.Sprite`))
  (:`Pressed`
    (set `self.IsAttack` true)
    (`PaperFlipbookComponent.SetFlipbook` _sprite "/Game/game_01/PaperaAssets/Character/LightMag/Flipbook/PF_Light_ball.PF_Light_ball")
    (`KismetSystemLibrary.Delay` (/ (`PaperFlipbookComponent.GetFlipbookLength` _sprite) 2.0))
    (bind _returnvalue (`|SpawnActorFromClass` "/Game/game_01/Blueprint/BP_Charge.BP_Charge_C" (`self.GetTransform`) "Undefined" "MultiplyWithRoot" null null))
    (set `/Game/game_01/Blueprint/BP_Charge.Dir` (`KismetMathLibrary.SelectFloat` -1.0 1.0 (`self.Dir`)) _returnvalue)
    (set `self.IsAttack` false)))

(fn `AnimationUpdate`
  (bind (_returnvalue_x _returnvalue_y _returnvalue_z) (`KismetMathLibrary.BreakVector` (`self.GetVelocity`)))
  (bind _sprite (`self.Sprite`))
  (if (`NavMovementComponent.IsMovingOnGround` (`self.CharacterMovement`))
    (if (> (`KismetMathLibrary.VSize` (`self.GetVelocity`)) 0.0)
      (`PaperFlipbookComponent.SetFlipbook` _sprite "/Game/game_01/PaperaAssets/Character/LightMag/Flipbook/PF_Run.PF_Run")
      (else
        (`PaperFlipbookComponent.SetFlipbook` _sprite "/Game/game_01/PaperaAssets/Character/LightMag/Flipbook/PF_Idle.PF_Idle")))
    (elif (> _returnvalue_z 100.0)
      (`PaperFlipbookComponent.SetFlipbook` (`self.Sprite`) "/Game/game_01/PaperaAssets/Character/LightMag/Flipbook/PF_Jump_Rise.PF_Jump_Rise")
      (else
        (`PaperFlipbookComponent.SetFlipbook` (`self.Sprite`) "/Game/game_01/PaperaAssets/Character/LightMag/Flipbook/PF_Jump_Down.PF_Jump_Down")))))

(fn `UserConstructionScript`)